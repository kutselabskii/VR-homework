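; Paladin is an AI-moved character that travels a route of three targets while the player pawn is more than 500 units away.
; Movement chains MoveTo calls with random walk speeds and delays, adding a jump before the final leg.
; MoveTo wraps AIMoveTo and skips new moves when CanMove is false.
; Tick updates CanMove from player distance and restarts Movement when the route ends or the player moves away.
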(event `self.ReceiveBeginPlay`
  (`self.Movement`))

(event `self.ReceiveTick`
  (params (DeltaSeconds :type "Float (single-precision)"))
  (bind _returnvalue (> (`self.GetDistanceTo` (`GameplayStatics.GetPlayerPawn` 0) self) 500.0))
  (if (`self.CanMove`)
    (set `self.CanMove` _returnvalue)
    (if (not (`self.Moving`))
      (`self.Movement`))
    (elif _returnvalue
      (set `self.CanMove` _returnvalue)
      (`self.Movement`))))

(fn `UserConstructionScript`)
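; ChaoticObject is a grabbable, breakable object with a static mesh and a Chaos geometry collection.
; A trace grip press calls Hold when the gripping object is close enough to the static mesh, and release calls Drop.
; When the geometry collection reports a Chaos break event, the Breaker component moves to the break location and activates.
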(event `self.TraceGripDown`
  (params (Object :type "SceneComponent Object Reference"))
  (if (< (`KismetMathLibrary.Vector_Distance` (`SceneComponent.K2_GetComponentLocation` Object) (`SceneComponent.K2_GetComponentLocation` (`self.StaticMeshComponent`))) 150.0)
    (`self.Hold` Object)))

(event `self.TraceGripUp`
  (params (Object :type "SceneComponent Object Reference"))
  (`self.Drop`))

(event `self.GeometryCollection.OnChaosBreakEvent`
  (params (BreakEvent :type "ChaosBreakEvent Structure (by ref)"))
  (bind _breaker (`self.Breaker`))
  (`SceneComponent.K2_SetWorldLocation` _breaker BreakEvent_Location false false)
  (`ActorComponent.Activate` _breaker false))

(fn `UserConstructionScript`)
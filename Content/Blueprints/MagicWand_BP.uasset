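; MagicWand_BP is a magic wand that can be picked up and fires a Lightning effect.
; On grip down it calls Hold if the passed Object is within 150 units of its static mesh and sets Gripped; grip up calls Drop and clears it.
; Trigger down activates Lightning whether or not the wand is held, as the Gripped check is not wired in.
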(event `self.ReceiveBeginPlay`
  (set `self.Gripped` false))

(event `self.TraceGripDown`
  (params (Object :type "SceneComponent Object Reference"))
  (if (< (`KismetMathLibrary.Vector_Distance` (`SceneComponent.K2_GetComponentLocation` Object) (`SceneComponent.K2_GetComponentLocation` (`self.StaticMeshComponent`))) 150.0)
    (`self.Hold` Object)
    (set `self.Gripped` true)))

(event `self.TraceGripUp`
  (params (Object :type "SceneComponent Object Reference"))
  (`self.Drop`)
  (set `self.Gripped` false))

(event `self.TraceTriggerDown`
  (`ActorComponent.Activate` (`self.Lightning`) false))

(fn `UserConstructionScript`)
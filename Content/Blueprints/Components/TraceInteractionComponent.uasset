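; Component that lets its owner point at and activate world objects by tracing forward from its location.
; While its gate is enabled, each tick runs either a straight line trace or a segmented, gravity-curved parabolic trace.
; Hit changes send move, enter and leave messages to TraceInteractionInterface actors per object and component, plus selection messages to InteractiveObject actors.
; ActivateDown and ActivateUp forward presses to the focused object.
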(event `self.ReceiveTick`
  (params (DeltaSeconds :type "Float (single-precision)"))
  (`/Engine/EditorBlueprintResources/StandardMacros.Gate` false :!label _label
    (:`Exit`
      (if (`self.UseLineTrace`)
        (bind _hit (`self.LineTrace` 1000.0))
        (bind _output_get (set `self.CurrentHit` _hit))
        (`self.InteractWithHit` _output_get)
        (`self.InteractWithInteractiveObject` _output_get)
        (else
          (bind _hit_2 (`self.ParabolicTrace` 50 0.05 (`self.ParabolicTraceSpeed`)))
          (bind _output_get_2 (set `self.CurrentHit` _hit_2))
          (`self.InteractWithHit` _output_get_2)
          (`self.InteractWithInteractiveObject` _output_get_2))))))

(event `Enable`
  (goto _label :!via `Open`))

(event `Disable`
  (goto _label :!via `Close`))

(event `ActivateDown`
  (params (Instigator :type "Pawn Object Reference"))
  (bind _focusedobject (`self.FocusedObject`))
  (message `/Game/Blueprints/Interfaces/TraceInteractionInterface.TraceActivateDown` _focusedobject (`self.CurrentHit`) Instigator)
  (message `InteractiveObject.Activated` _focusedobject))

(event `ActivateUp`
  (params (Instigator :type "Pawn Object Reference"))
  (message `/Game/Blueprints/Interfaces/TraceInteractionInterface.TraceActivateUp` (`self.FocusedObject`) (`self.CurrentHit`) Instigator))

(fn `InteractWithHit`
  (params (Hit :type "HitResult Structure"))
  (locals (inHit :type "HitResult Structure") (inHitActor :type "Actor Object Reference") (inHitComponent :type "PrimitiveComponent Object Reference"))
  (bind _inhitactor (`local.inHitActor`))
  (bind _output_get (set `local.inHit` Hit))
  (bind (_bblockinghit _binitialoverlap _time _distance _location _impactpoint _normal _impactnormal _physmat _hitactor _hitcomponent) (`GameplayStatics.BreakHitResult` _output_get))
  (set `local.inHitActor` _hitactor)
  (set `local.inHitComponent` _hitcomponent)
  (if (== (`local.inHitActor`) (`self.FocusedObject`))
    (message `/Game/Blueprints/Interfaces/TraceInteractionInterface.TraceMove` (`self.FocusedObject`) (`local.inHit`))
    (if (not (== (`self.FocusedComponent`) (`local.inHitComponent`)))
      (message `/Game/Blueprints/Interfaces/TraceInteractionInterface.TraceLeaveComponent` (`self.FocusedObject`) (`local.inHit`) (`self.FocusedComponent`))
      (message `/Game/Blueprints/Interfaces/TraceInteractionInterface.TraceHitComponent` (`self.FocusedObject`) (`local.inHit`) (`local.inHitComponent`))
      (set `self.FocusedComponent` (`local.inHitComponent`)))
    (else
      (message `/Game/Blueprints/Interfaces/TraceInteractionInterface.TraceLeaveObject` (`self.FocusedObject`) (`local.inHit`))
      (set `self.FocusedObject` null)
      (set `self.FocusedComponent` null)
      (if (`KismetSystemLibrary.DoesImplementInterface` (`local.inHitActor`) "/Game/Blueprints/Interfaces/TraceInteractionInterface.TraceInteractionInterface_C")
        (message `/Game/Blueprints/Interfaces/TraceInteractionInterface.TraceHitObject` (`local.inHitActor`) (`local.inHit`))
        (message `/Game/Blueprints/Interfaces/TraceInteractionInterface.TraceHitComponent` (`local.inHitActor`) (`local.inHit`) (`local.inHitComponent`))
        (set `self.FocusedObject` (`local.inHitActor`))
        (set `self.FocusedComponent` (`local.inHitComponent`))
        (if (`KismetSystemLibrary.DoesImplementInterface` _inhitactor "/Script/Simple_movement.InteractiveObject")
          (message `InteractiveObject.Selected` _inhitactor))))))

(fn `InteractWithInteractiveObject`
  (params (Hit :type "HitResult Structure"))
  (bind (_bblockinghit _binitialoverlap _time _distance _location _impactpoint _normal _impactnormal _physmat _hitactor) (`GameplayStatics.BreakHitResult` Hit))
  (if (`KismetSystemLibrary.DoesImplementInterface` _hitactor "/Script/Simple_movement.InteractiveObject")
    (if (not (== (`self.FocusedObject`) _hitactor))
      (message `InteractiveObject.Selected` _hitactor))))

(fn `LineTrace`
  (params (Distance :type "Float (double-precision)"))
  (returns (Hit :type "HitResult Structure"))
  (bind _returnvalue (`self.K2_GetComponentLocation`))
  (bind _outhit (`KismetSystemLibrary.LineTraceSingle` :`Start` _returnvalue :`End` (+ _returnvalue (* (`self.GetForwardVector`) Distance)) :`TraceChannel` "TraceTypeQuery1" :`DrawDebugType` (`self.TraceDrawDebugType`)))
  (return _outhit))

(fn `ParabolicTrace`
  (params (Steps :type Integer) (TimeStep :type "Float (double-precision)") (Speed :type "Float (double-precision)"))
  (returns (Hit :type "HitResult Structure"))
  (locals (InitialLocation :type "Vector Structure") (PreviousLocation :type "Vector Structure") (Velocity :type "Vector Structure") (InTimeStep :type "Float (double-precision)") (InSteps :type Integer) (TmpHit :type "HitResult Structure"))
  (bind (_velocity_x _velocity_y _velocity_z) (`KismetMathLibrary.BreakVector` (`local.Velocity`)))
  (bind _output_get (set `local.InitialLocation` (`self.K2_GetComponentLocation`)))
  (set `local.PreviousLocation` _output_get)
  (set `local.InSteps` Steps)
  (set `local.InTimeStep` TimeStep)
  (set `local.Velocity` (* (`KismetMathLibrary.Conv_DoubleToVector` Speed) (`self.GetForwardVector`)))
  (for _index (range 1 (+ (`local.InSteps`) 1))
    (bind _returnvalue (* _index (`local.InTimeStep`)))
    (bind _returnvalue_2 (+ (`KismetMathLibrary.MakeVector` (* _velocity_x _returnvalue) (* _velocity_y _returnvalue) (- (* _velocity_z _returnvalue) (* _returnvalue _returnvalue 0.5 980.0))) (`local.InitialLocation`)))
    (bind (_outhit _returnvalue_3) (`KismetSystemLibrary.LineTraceSingle` :`Start` (`local.PreviousLocation`) :`End` _returnvalue_2 :`TraceChannel` "TraceTypeQuery1" :`DrawDebugType` (`self.TraceDrawDebugType`)))
    (set `local.PreviousLocation` _returnvalue_2)
    (set `local.TmpHit` _outhit)
    (if _returnvalue_3
      (break)))
  (return (`local.TmpHit`)))
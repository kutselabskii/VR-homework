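; Ignitor is a grippable actor with a Fire component that can be lit and put out.
; Ignite activates Fire and records the time, and Tick deactivates it five seconds after the latest ignition.
; Choke extinguishes it immediately.
; Trace grip events call Hold when the gripping object is within range of the static mesh, and Drop on release.
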(event `self.ReceiveBeginPlay`
  (set `self.IngitionTime` (`KismetMathLibrary.DateTimeMinValue`)))

(event `self.ReceiveTick`
  (params (DeltaSeconds :type "Float (single-precision)"))
  (bind _fire (`self.Fire`))
  (if (and (>= (- (`KismetMathLibrary.Now`) (`self.IngitionTime`)) (`KismetMathLibrary.MakeTimespan` 0 0 0 5)) (`ActorComponent.IsActive` _fire))
    (`ActorComponent.Deactivate` _fire)))

(event `self.TraceGripDown`
  (params (Object :type "SceneComponent Object Reference"))
  (if (< (`KismetMathLibrary.Vector_Distance` (`SceneComponent.K2_GetComponentLocation` Object) (`SceneComponent.K2_GetComponentLocation` (`self.StaticMeshComponent`))) 150.0)
    (`self.Hold` Object)))

(event `self.TraceGripUp`
  (params (Object :type "SceneComponent Object Reference"))
  (`self.Drop`))

(fn `Choke`
  (bind _fire (`self.Fire`))
  (if (`ActorComponent.IsActive` _fire)
    (`ActorComponent.Deactivate` _fire)))

(fn `Ignite`
  (bind _fire (`self.Fire`))
  (if (not (`ActorComponent.IsActive` _fire))
    (`ActorComponent.Activate` _fire false))
  (set `self.IngitionTime` (`KismetMathLibrary.Now`)))

(fn `UserConstructionScript`)